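; Demo actor that shows relative-context bitmask queries between itself and the player's controlled pawn.
; BeginPlay caches the first player controller, and the CalculateRelativeContext event stores the actor's context relative to that controller's pawn as a bitmask.
; Tick tests the stored value against a fixed flag and prints the result on screen; nothing in this graph triggers the recalculation.
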(event EventBeginPlay
  (Variables|Default|SetCharacterReference (Game|GetPlayerController 0)))

(event Collision|EventActorBeginOverlap
  (params (OtherActor :type Actor%20Object%20Reference)))

(event EventTick
  (params (DeltaSeconds :type Float%20%28single-precision%29))
  (bind _returnvalue (Class|SpatialContextLibrary|TestRelativeContext (|BitmaskLiteral 64) (Variables|Default|GetRelativeContext)))
  (Development|PrintString (Utilities|String|ToString(Boolean) _returnvalue) true true "(R=0.000000,G=0.660000,B=1.000000,A=1.000000)" 0.01 "1"))

(event EventCalculateRelativeContext
  (bind _returnvalue (Class|SpatialContextLibrary|GetRelativeContext self (Pawn|GetControlledPawn (Variables|Default|GetCharacterReference))))
  (Variables|Default|SetRelativeContext (|BitmaskLiteral _returnvalue)))

(fn ConstructionScript)